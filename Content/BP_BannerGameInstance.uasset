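; BP_BannerGameInstance is a game instance that owns the player's persistent banner save and exposes the selected banner.
; On Init it loads the "Banner" save slot as BP_BannerSave, creating a fresh save object if that fails, and a SaveGame event writes it back to the same slot.
; GetSelectedBanner uses the saved selection as a row name to return the matching BannerConfig data table row.
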(event Custom|SaveGame
  (SaveGame|SaveGametoSlot (Variables|Default|GetSave) "Banner"))

(event EventInit
  (bind _returnvalue (SaveGame|LoadGamefromSlot "Banner"))
  (bind _asbp_banner_save (Utilities|Casting|CastToBP_BannerSave _returnvalue)
    (:then
      (Variables|Default|SetSave _asbp_banner_save))
    (:CastFailed
      (bind _returnvalue_2 (SaveGame|CreateSaveGameObject "/Game/BP_BannerSave.BP_BannerSave_C"))
      (Variables|Default|SetSave _returnvalue_2))))

(fn GetSelectedBanner
  (bind _returnvalue (Utilities|GetDataTableRow "/Game/BannerConfig.BannerConfig" (Utilities|String|StringToName (Variables|/Game/BP_BannerSave.BP_BannerSave_C|GetSelectedBanner (Variables|Default|GetSave))))
    (:then
      (return _returnvalue))
    (:RowNotFound
      (return ""))))